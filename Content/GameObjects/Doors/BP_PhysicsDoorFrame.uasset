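; Physics door that an interactor pushes or pulls, alerting monsters with noise.
; Server_Interact applies a mass-scaled impulse to Frame along the interactor capsule's forward vector, reversed when IsPush is false.
; It then gathers every BP_MonsterCharacter and passes them to the server noise event, which prints a "CREEK" debug string and sends each an EmitNoiseMessage with the door's location and loudness.
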(event Custom|Server_Interact
  (params (Interactor :type BP%20First%20Person%20Character%20Object%20Reference))
  (bind _capsulecomponent (Variables|/Script/Engine.Character|GetCapsuleComponent Interactor))
  (bind _movementforce (Variables|Default|GetMovementForce))
  (bind _frame (Variables|Default|GetFrame))
  (bind _returnvalue (Physics|GetMass _frame))
  (bind _returnvalue_2 (Math|Vector|GetForwardVector _capsulecomponent))
  (bind _returnvalue_3 (* _movementforce _returnvalue))
  (bind _returnvalue_4 (* _returnvalue_3 _returnvalue_2))
  (if (Variables|Default|GetbIsPush)
    (Physics|AddImpulse (Variables|Default|GetFrame) _returnvalue_4 "None" false)
    (else
      (Physics|AddImpulse (Variables|Default|GetFrame) (* _returnvalue_4 "-1.000000,-1.000000,-1.000000") "None" false)))
  (bind _outactors (Actor|GetAllActorsOfClass "/Game/AI/BP_MonsterCharacter.BP_MonsterCharacter_C"))
  (CallFunction|ServerEmitNoise _outactors (Transformation|GetActorLocation) (Variables|Default|GetLoudness)))

(event Custom|Server_EmitNoise
  (params (Targets :type Array%20of%20Actor%20Object%20References) (Location :type Vector) (Loudness :type Float%20%28double-precision%29))
  (Development|PrintString "CREEK")
  (Class|BPINoiseEmitter|EmitNoise(Message) Targets Location Loudness))

(fn ConstructionScript)