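; Table furniture Blueprint that defines where objects can spawn on it.
; It overrides SetupSpawnPoints, calls the parent version, then writes two spawn point structs into the SpawnPoints array, each tying a component to an allowed size and rare chance.
; The event graph holds only disabled stubs, and the construction script just defers to the parent.
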(event EventBeginPlay
  (|CallParentFunction) ; This node is disabled and will not be called.\nDrag off pins to build functionality.
)

(event Collision|EventActorBeginOverlap
  (params (OtherActor :type Actor%20Object%20Reference)))

(event EventTick
  (params (DeltaSeconds :type Float%20%28single-precision%29)))

(fn ConstructionScript
  (|CallParentFunction))

(fn SetupSpawnPoints
  (|CallParentFunction)
  (Utilities|Array|SetArrayElem (Variables|Default|GetSpawnPoints) 1 (Utilities|Struct|MakeS_ObjectSpawnPoint (Variables|Default|GetSpawnPoint) "NewEnumerator1" 1.0))
  (Utilities|Array|SetArrayElem (Variables|Default|GetSpawnPoints) 0 (Utilities|Struct|MakeS_ObjectSpawnPoint (Variables|Default|GetSpawnPoint1) "NewEnumerator0" 1.0)))