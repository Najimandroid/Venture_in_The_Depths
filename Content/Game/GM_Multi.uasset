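; Multiplayer game mode that populates furniture with holdable objects on the server, five seconds after play begins.
; It gathers spawn points from every BP_FurnitureBase, separating forced points from optional ones.
; Forced points always spawn a BP_HoldableObject, then shuffled optional points fill up to a target total that counts the forced spawns.
; Used points are flagged; AllowedSize and RareChance are carried along but never affect spawning.
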(event Custom|Server_SetupAllSpawnPoints
  (bind _outactors (Actor|GetAllActorsOfClass "/Game/Blueprints/Furnitures/BP_FurnitureBase.BP_FurnitureBase_C"))
  (for _array_element _outactors
    (for _array_element_2 (Variables|/Game/Blueprints/Furnitures/BP_FurnitureBase.BP_FurnitureBase_C|GetSpawnPoints _array_element)
      (if (.bForceSpawn (Utilities|Struct|BreakS_ObjectSpawnPoint _array_element_2))
        (Utilities|Array|Add (Variables|Default|GetSpawnPointsToUse) _array_element_2)
        (else
          (Utilities|Array|Add (Variables|Default|GetSpawnPointsAvailableToUse) _array_element_2)))))
  (CallFunction|ServerSpawnObjects 10))

(event Custom|Server_SpawnObjects
  (params (NumberOfObjects :type Integer))
  (bind _spawnpointsavailabletouse (Variables|Default|GetSpawnPointsAvailableToUse))
  (bind _spawnpointstouse (Variables|Default|GetSpawnPointsToUse))
  (for (_array_element _array_index) _spawnpointstouse
    (CallFunction|SpawnObjectatPoint (.SpawnComponent (Utilities|Struct|BreakS_ObjectSpawnPoint _array_element)))
    (Utilities|Array|SetArrayElem _spawnpointstouse _array_index (Utilities|Struct|MakeS_ObjectSpawnPoint (.SpawnComponent (Utilities|Struct|BreakS_ObjectSpawnPoint _array_element)) (.AllowedSize (Utilities|Struct|BreakS_ObjectSpawnPoint _array_element)) (.RareChance (Utilities|Struct|BreakS_ObjectSpawnPoint _array_element)) (.bForceSpawn (Utilities|Struct|BreakS_ObjectSpawnPoint _array_element)) true)))
  (Utilities|Array|Shuffle _spawnpointsavailabletouse)
  (bind (_array_element_2 _array_index_2) (Utilities|Array|ForEachLoopwithBreak _spawnpointsavailabletouse :!label _label)
    (:LoopBody
      (if (>= (Variables|Default|GetSpawnedObjects) NumberOfObjects)
        (goto _label Break)
        (elif (== (.bAlreadyUsed (Utilities|Struct|BreakS_ObjectSpawnPoint _array_element_2)) false)
          (CallFunction|SpawnObjectatPoint (.SpawnComponent (Utilities|Struct|BreakS_ObjectSpawnPoint _array_element_2)))
          (Utilities|Array|SetArrayElem _spawnpointsavailabletouse _array_index_2 (Utilities|Struct|MakeS_ObjectSpawnPoint (.SpawnComponent (Utilities|Struct|BreakS_ObjectSpawnPoint _array_element_2)) (.AllowedSize (Utilities|Struct|BreakS_ObjectSpawnPoint _array_element_2)) (.RareChance (Utilities|Struct|BreakS_ObjectSpawnPoint _array_element_2)) (.bForceSpawn (Utilities|Struct|BreakS_ObjectSpawnPoint _array_element_2)) true)))))))

(event Custom|Server_StartGame
  (Networking|SwitchHasAuthority
    (:Authority
      (CallFunction|ServerSetupAllSpawnPoints))))

(event EventBeginPlay
  (Utilities|FlowControl|Delay 5.0)
  (CallFunction|ServerStartGame))

(fn ConstructionScript
  (|CallParentFunction))

(fn SpawnObjectatPoint
  (params (SpawnComponent :type Scene%20Component%20Object%20Reference))
  (Variables|Default|SetSpawnedObjects (+ (Variables|Default|GetSpawnedObjects) 1))
  (Game|SpawnActorfromClass "/Game/Blueprints/Objects/BP_HoldableObject.BP_HoldableObject_C" (Math|Conversions|ToTransform(Vector) (Transformation|GetWorldLocation SpawnComponent)) "Undefined" "MultiplyWithRoot" 0 0))