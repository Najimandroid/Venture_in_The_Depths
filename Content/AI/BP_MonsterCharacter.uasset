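; Monster AI character that hunts the first-person player by sight and sound, and triggers the player's server-side elimination on collision-box overlap.
; Pawn sensing writes the seen player to the blackboard as the target, and a retriggerable delay clears it once sightings stop.
; Noise events treat loudness as hearing radius and, when no target exists, write the heard location and flag to the blackboard.
; The construction script derives movement speeds from WalkSpeed.
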(event OnSeePawn(PawnSensing)
  (params (Pawn :type Pawn%20Object%20Reference))
  (bind _asbp_first_person_character (Utilities|Casting|CastToBP_FirstPersonCharacter Pawn))
  (Variables|Default|SetbIsChasingPlayer true)
  (Utilities|FlowControl|Sequence
    (:then_0
      (bind _output_get (Variables|Default|SetCurrentTarget _asbp_first_person_character))
      (AI|Components|Blackboard|SetValueasObject (AI|GetBlackboard (Pawn|GetController)) (Variables|Default|GetTargetActorKey) _output_get))
    (:then_1
      (Utilities|FlowControl|RetriggerableDelay (Variables|Default|GetLookForDelay))
      (Variables|Default|SetbIsChasingPlayer false)
      (AI|Components|Blackboard|SetValueasObject (AI|GetBlackboard (Pawn|GetController)) (Variables|Default|GetTargetActorKey) 0))))

(event OnComponentBeginOverlap(CollisionBox)
  (params (OverlappedComponent :type Primitive%20Component%20Object%20Reference) (OtherActor :type Actor%20Object%20Reference) (OtherComp :type Primitive%20Component%20Object%20Reference) (OtherBodyIndex :type Integer) (bFromSweep :type Boolean) (SweepResult :type Hit%20Result%20Structure%20%28by%20ref%29))
  (bind _asbp_first_person_character (Utilities|Casting|CastToBP_FirstPersonCharacter OtherActor))
  (Default|ServerDetectElemination _asbp_first_person_character)
  (Development|PrintString "KILL" true true "(R=1.000000,G=0.003500,B=0.006342,A=1.000000)"))

(event EventEmitNoise
  (params (Location :type Vector :default "0, 0, 0") (Loudness :type Float%20%28double-precision%29))
  (CallFunction|ReceiveNoise Location Loudness))

(fn ConstructionScript
  (bind _charactermovement (Variables|Character|GetCharacterMovement))
  (bind _output_get (Variables|/Script/Engine.CharacterMovementComponent|SetMaxWalkSpeed _charactermovement (Variables|Default|GetWalkSpeed)))
  (Variables|/Script/Engine.CharacterMovementComponent|SetMaxWalkSpeedCrouched _charactermovement (/ _output_get 2.0)))

(fn ReceiveNoise
  (params (Location :type Vector) (Loudness :type Float%20%28double-precision%29))
  (bind _returnvalue (Pawn|GetController))
  (bind _returnvalue_2 (AI|GetBlackboard _returnvalue))
  (Development|PrintText "I HEARD A NOISE" true true "(R=1.000000,G=0.000000,B=0.009073,A=1.000000)")
  (if (<= (Math|Vector|Distance(Vector) (Transformation|GetActorLocation) Location) Loudness)
    (if (not (Utilities|IsValid (AI|Components|Blackboard|GetValueasObject _returnvalue_2 (Variables|Default|GetTargetActorKey))))
      (bind _output_get (Variables|Default|SetLastHeardLocation Location))
      (AI|Components|Blackboard|SetValueasVector _returnvalue_2 (Variables|Default|GetMoveLocationKey) _output_get)
      (AI|Components|Blackboard|SetValueasBool _returnvalue_2 (Variables|Default|GetHasHeardNoiseKey) true))))