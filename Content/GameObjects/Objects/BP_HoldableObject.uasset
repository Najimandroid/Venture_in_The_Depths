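; Replicated physics object that players can pick up, carry, drop and throw, alerting monsters on impact.
; Server-authoritative Pickup and Drop set owner and held state, whose RepNotifies toggle collision, physics and material.
; While held, the locally controlled owner interpolates it along the camera aim each tick and forwards its location to the server.
; Hits far enough from the last held position send noise to all BP_MonsterCharacters, currently at world origin.
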(event OnComponentHit(SphereCollision)
  (params (HitComponent :type Primitive%20Component%20Object%20Reference) (OtherActor :type Actor%20Object%20Reference) (OtherComp :type Primitive%20Component%20Object%20Reference) (NormalImpulse :type Vector :default "0, 0, 0") (Hit :type Hit%20Result%20Structure%20%28by%20ref%29))
  (bind _impactpoint (Collision|BreakHitResult Hit))
  (bind _lastheldposition (Variables|Default|GetLastHeldPosition))
  (bind _returnvalue (Math|Vector|Distance(Vector) _lastheldposition _impactpoint))
  (Development|PrintString (Utilities|String|ToString(Float) _returnvalue))
  (if (>= _returnvalue 3e+01)
    (bind _outactors (Actor|GetAllActorsOfClass "/Game/AI/BP_MonsterCharacter.BP_MonsterCharacter_C"))
    (CallFunction|ServerEmitNoise _outactors "0, 0, 0" (Variables|Default|GetDropLoudness))))

(event Custom|Server_EmitNoise
  (params (Targets :type Array%20of%20Actor%20Object%20References) (Location :type Vector) (Loudness :type Float%20%28double-precision%29))
  (Development|PrintString "BOOM")
  (Class|BPINoiseEmitter|EmitNoise(Message) Targets Location Loudness))

(event Custom|Server_RequestPickup
  (params (PlayerState :type Player%20State%20Object%20Reference))
  (CallFunction|Pickup PlayerState))

(event Custom|Server_UpdateObjectLocation
  (params (NewLocation :type Vector))
  (Networking|SwitchHasAuthority
    (:Authority
      (Transformation|SetActorLocation NewLocation false false))))

(event Custom|Server_RequestDrop
  (params (PlayerState :type Player%20State%20Object%20Reference))
  (CallFunction|Drop PlayerState))

(event EventTick
  (params (DeltaSeconds :type Float%20%28single-precision%29))
  (if (Variables|Default|GetbIsHeld)
    (if (Pawn|IsLocallyControlled (PlayerState|GetPawn (Variables|Default|GetCurrentOwner)))
      (CallFunction|UpdateHoldPosition DeltaSeconds))))

(fn ConstructionScript)

(fn OnRepPriceValue)

(fn OnRepCurrentOwner
  (if (Utilities|IsValid (Variables|Default|GetCurrentOwner))
    (Rendering|Material|SetMaterial (Variables|Default|GetMesh) 0 "/Game/FirstPerson/MI_FirstPersonColorway.MI_FirstPersonColorway")
    (else
      (Rendering|Material|SetMaterial (Variables|Default|GetMesh) 0 "/Game/LevelPrototyping/Materials/M_FlatCol.M_FlatCol"))))

(fn OnRepBIsHeld
  (if (Variables|Default|GetbIsHeld)
    (if true
      (Transformation|DetachFromActor "KeepWorld" "KeepWorld" "KeepRelative")
      (Collision|SetCollisionEnabled (Variables|Default|GetSphereCollision) "NoCollision"))
    (else
      (Physics|SetSimulatePhysics (Variables|Default|GetSphereCollision) true)
      (Collision|SetCollisionEnabled (Variables|Default|GetSphereCollision) "QueryAndPhysics"))))

(fn Pickup
  (params (PlayerState :type Player%20State%20Object%20Reference))
  ;[0.15 0.15 0.15 0.5] Checks if we are currently executing in the server
  (Networking|SwitchHasAuthority
    (:Authority
      ;[0.15 0.15 0.15 0.5] Checks if the object is not locked
      (if (not (Variables|Default|GetbIsLocked))
        (if (not (Variables|Default|GetbIsHeld))
          (Variables|Default|SetbIsLocked true)
          (Variables|Default|SetCurrentOwner PlayerState)
          (Variables|Default|SetbIsHeld true)
          (bind _asbp_first_person_character (Utilities|Casting|CastToBP_FirstPersonCharacter (PlayerState|GetPawn PlayerState)))
          (Variables|/Game/FirstPerson/Blueprints/BP_FirstPersonCharacter.BP_FirstPersonCharacter_C|SetHeldObject _asbp_first_person_character self)
          (Variables|Default|SetbIsLocked false))))))

(fn Drop
  (params (PlayerState :type Player%20State%20Object%20Reference))
  ;[0.15 0.15 0.15 0.5] Checks if we are currently executing in the server
  (Networking|SwitchHasAuthority
    (:Authority
      ;[0.15 0.15 0.15 0.5] Checks if the object is dropped by the player
      (if (== (Variables|Default|GetCurrentOwner) PlayerState)
        (if (Variables|Default|GetbIsHeld)
          (Variables|Default|SetbIsHeld false)
          (Variables|Default|SetCurrentOwner 0)
          (bind _asbp_first_person_character (Utilities|Casting|CastToBP_FirstPersonCharacter (PlayerState|GetPawn PlayerState)))
          (Variables|/Game/FirstPerson/Blueprints/BP_FirstPersonCharacter.BP_FirstPersonCharacter_C|SetHeldObject _asbp_first_person_character 0))))))

(fn UpdateHoldPosition
  (params (DeltaTime :type Float%20%28double-precision%29))
  (bind _self self)
  (bind _holddistance (Variables|Default|GetHoldDistance))
  ;[0.15 0.15 0.15 0.5] Casting the current owner to BP_FirstPersonCharacter
  (bind _asbp_first_person_character (Utilities|Casting|CastToBP_FirstPersonCharacter (PlayerState|GetPawn (Variables|Default|GetCurrentOwner))))
  ;[0.15 0.15 0.15 0.5] Setting the new location and rotation smoothly
  (Transformation|SetActorLocation _self (Math|Interpolation|VInterpTo (Transformation|GetActorLocation _self) (+ (Transformation|GetWorldLocation (Variables|/Game/FirstPerson/Blueprints/BP_FirstPersonCharacter.BP_FirstPersonCharacter_C|GetFirstPersonCamera _asbp_first_person_character)) (* (Math|Vector|GetForwardVector (Math|Rotator|MakeRotator 0.0 (Variables|/Game/FirstPerson/Blueprints/BP_FirstPersonCharacter.BP_FirstPersonCharacter_C|GetReplicatedAimPitch _asbp_first_person_character) (.Yaw (Math|Rotator|BreakRotator (Transformation|GetWorldRotation (Variables|/Game/FirstPerson/Blueprints/BP_FirstPersonCharacter.BP_FirstPersonCharacter_C|GetFirstPersonCamera _asbp_first_person_character)))))) (Math|Vector|MakeVector _holddistance _holddistance _holddistance))) DeltaTime (Variables|Default|GetHoldInterpSpeed)) false false)
  (Transformation|SetActorRotation (Math|Rotator|MakeRotator 0.0 (Variables|/Game/FirstPerson/Blueprints/BP_FirstPersonCharacter.BP_FirstPersonCharacter_C|GetReplicatedAimPitch _asbp_first_person_character) (.Yaw (Math|Rotator|BreakRotator (Transformation|GetWorldRotation (Variables|/Game/FirstPerson/Blueprints/BP_FirstPersonCharacter.BP_FirstPersonCharacter_C|GetFirstPersonCamera _asbp_first_person_character))))))
  (Variables|Default|SetLastHeldPosition (Math|Interpolation|VInterpTo (Transformation|GetActorLocation _self) (+ (Transformation|GetWorldLocation (Variables|/Game/FirstPerson/Blueprints/BP_FirstPersonCharacter.BP_FirstPersonCharacter_C|GetFirstPersonCamera _asbp_first_person_character)) (* (Math|Vector|GetForwardVector (Math|Rotator|MakeRotator 0.0 (Variables|/Game/FirstPerson/Blueprints/BP_FirstPersonCharacter.BP_FirstPersonCharacter_C|GetReplicatedAimPitch _asbp_first_person_character) (.Yaw (Math|Rotator|BreakRotator (Transformation|GetWorldRotation (Variables|/Game/FirstPerson/Blueprints/BP_FirstPersonCharacter.BP_FirstPersonCharacter_C|GetFirstPersonCamera _asbp_first_person_character)))))) (Math|Vector|MakeVector _holddistance _holddistance _holddistance))) DeltaTime (Variables|Default|GetHoldInterpSpeed)))
  ;[0.15 0.15 0.15 0.5] Forwarding the location value to the server
  (Default|ServerTryUpdateObjectLocation _asbp_first_person_character self (Math|Interpolation|VInterpTo (Transformation|GetActorLocation _self) (+ (Transformation|GetWorldLocation (Variables|/Game/FirstPerson/Blueprints/BP_FirstPersonCharacter.BP_FirstPersonCharacter_C|GetFirstPersonCamera _asbp_first_person_character)) (* (Math|Vector|GetForwardVector (Math|Rotator|MakeRotator 0.0 (Variables|/Game/FirstPerson/Blueprints/BP_FirstPersonCharacter.BP_FirstPersonCharacter_C|GetReplicatedAimPitch _asbp_first_person_character) (.Yaw (Math|Rotator|BreakRotator (Transformation|GetWorldRotation (Variables|/Game/FirstPerson/Blueprints/BP_FirstPersonCharacter.BP_FirstPersonCharacter_C|GetFirstPersonCamera _asbp_first_person_character)))))) (Math|Vector|MakeVector _holddistance _holddistance _holddistance))) DeltaTime (Variables|Default|GetHoldInterpSpeed))))

(fn ThrowObject
  (params (Force :type Float%20%28double-precision%29))
  ;[0.15 0.15 0.15 0.5] Casting the current owner to BP_FirstPersonCharacter
  (bind _asbp_first_person_character (Utilities|Casting|CastToBP_FirstPersonCharacter (PlayerState|GetPawn (Variables|Default|GetCurrentOwner))))
  (Physics|AddImpulse (Variables|Default|GetSphereCollision) (+ (Transformation|GetWorldLocation (Variables|/Game/FirstPerson/Blueprints/BP_FirstPersonCharacter.BP_FirstPersonCharacter_C|GetFirstPersonCamera _asbp_first_person_character)) (* (Math|Vector|GetForwardVector (Math|Rotator|MakeRotator 0.0 (Variables|/Game/FirstPerson/Blueprints/BP_FirstPersonCharacter.BP_FirstPersonCharacter_C|GetReplicatedAimPitch _asbp_first_person_character) (.Yaw (Math|Rotator|BreakRotator (Transformation|GetWorldRotation (Variables|/Game/FirstPerson/Blueprints/BP_FirstPersonCharacter.BP_FirstPersonCharacter_C|GetFirstPersonCamera _asbp_first_person_character)))))) (Math|Vector|MakeVector Force Force Force))) "None" false))