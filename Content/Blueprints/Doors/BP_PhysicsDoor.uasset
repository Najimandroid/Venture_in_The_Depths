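; BP_PhysicsDoor is a networked physics door that one player at a time can hold.
; Interact, only on non-authority instances, sends the player's PlayerState to a server request that toggles the hold and ignores other players while held.
; The server also sets the character's AlreadyOnHold flag.
; The IsHeld RepNotify switches the Axis constraint's swing between limited while held and locked when released.
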(event Custom|Server_RequestHold
  (params (PlayerState :type Player%20State%20Object%20Reference))
  (if (Variables|Default|GetbIsHeld)
    (if (== (Variables|Default|GetCurrentHolder) PlayerState)
      (Variables|Default|SetbIsHeld false)
      (bind _asbp_first_person_character (Utilities|Casting|CastToBP_FirstPersonCharacter (PlayerState|GetPawn (Variables|Default|GetCurrentHolder))))
      (Variables|/Game/FirstPerson/Blueprints/BP_FirstPersonCharacter.BP_FirstPersonCharacter_C|SetbAlreadyOnHold _asbp_first_person_character false)
      (Variables|Default|SetCurrentHolder 0))
    (else
      (Variables|Default|SetbIsHeld true)
      (Variables|Default|SetCurrentHolder PlayerState)
      (bind _asbp_first_person_character_2 (Utilities|Casting|CastToBP_FirstPersonCharacter (PlayerState|GetPawn PlayerState)))
      (Variables|/Game/FirstPerson/Blueprints/BP_FirstPersonCharacter.BP_FirstPersonCharacter_C|SetbAlreadyOnHold _asbp_first_person_character_2 true))))

(fn ConstructionScript)

(fn OnRepBIsHeld
  (bind _axis (Variables|Default|GetAxis))
  (if (Variables|Default|GetbIsHeld)
    (Class|PhysicsConstraintComponent|SetAngularSwing1Limit _axis "ACM_Limited" 75.0)
    (else
      (Class|PhysicsConstraintComponent|SetAngularSwing1Limit _axis "ACM_Locked" 75.0))))

(fn Interact
  (params (Interactor :type BP%20First%20Person%20Character%20Object%20Reference))
  (Networking|SwitchHasAuthority
    (:Remote
      (CallFunction|ServerRequestHold (Variables|/Script/Engine.Pawn|GetPlayerState Interactor)))))