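; BP_ObjectSeller is a drop zone actor that turns holdable objects into money.
; When a BP_HoldableObject that is not held begins overlapping the DropZone, the server adds its PriceValue to MoneyPool and locks the object.
; MoneyPool's RepNotify fires the OnMoneyChanged dispatcher with the new total.
; A field-value broadcast for UW_GameplayScreen is present but unconnected.
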(event OnComponentBeginOverlap(DropZone)
  (params (OverlappedComponent :type Primitive%20Component%20Object%20Reference) (OtherActor :type Actor%20Object%20Reference) (OtherComp :type Primitive%20Component%20Object%20Reference) (OtherBodyIndex :type Integer) (bFromSweep :type Boolean) (SweepResult :type Hit%20Result%20Structure%20%28by%20ref%29))
  (Networking|SwitchHasAuthority
    (:Authority
      (bind _asbp_holdable_object (Utilities|Casting|CastToBP_HoldableObject OtherActor))
      (if (not (Variables|/Game/Blueprints/Objects/BP_HoldableObject.BP_HoldableObject_C|GetbIsHeld _asbp_holdable_object))
        (Variables|Default|SetMoneyPool (+ (Variables|Default|GetMoneyPool) (Variables|/Game/Blueprints/Objects/BP_HoldableObject.BP_HoldableObject_C|GetPriceValue _asbp_holdable_object)))
        (Variables|/Game/Blueprints/Objects/BP_HoldableObject.BP_HoldableObject_C|SetbIsLocked _asbp_holdable_object true)))))

(fn ConstructionScript)

(fn OnRepMoneyPool
  (Default|CallOnMoneyChanged (Variables|Default|GetMoneyPool)))