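; Networked physics object that BP_FirstPersonCharacter players can pick up and drop.
; Server request events call authority-only Pickup and Drop, which update held state, owning PlayerState and the character's HeldObject, with a lock guarding pickup.
; OnRep_bIsHeld toggles the sphere's physics and collision, attaching to the right-hand grip socket or detaching.
; OnRep_CurrentOwner swaps the cube's material to show ownership; PriceValue's OnRep is empty.
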(event Custom|Server_RequestPickup
  (params (PlayerState :type Player%20State%20Object%20Reference))
  (CallFunction|Pickup PlayerState))

(event Custom|Server_RequestDrop
  (params (PlayerState :type Player%20State%20Object%20Reference))
  (CallFunction|Drop PlayerState))

(fn ConstructionScript)

(fn OnRepPriceValue)

(fn OnRepCurrentOwner
  (if (Utilities|IsValid (Variables|Default|GetCurrentOwner))
    (Rendering|Material|SetMaterial (Variables|Default|GetCube) 0 "/Game/FirstPerson/MI_FirstPersonColorway.MI_FirstPersonColorway")
    (else
      (Rendering|Material|SetMaterial (Variables|Default|GetCube) 0 "/Game/LevelPrototyping/Materials/M_FlatCol.M_FlatCol"))))

(fn OnRepBIsHeld
  (bind _currentowner (Variables|Default|GetCurrentOwner))
  (if (Variables|Default|GetbIsHeld)
    (if (Utilities|IsValid _currentowner)
      (bind _asbp_first_person_character (Utilities|Casting|CastToBP_FirstPersonCharacter (PlayerState|GetPawn _currentowner)))
      (Physics|SetSimulatePhysics (Variables|Default|GetSphere) false)
      (Collision|SetCollisionEnabled (Variables|Default|GetSphere) "NoCollision")
      (Transformation|AttachActorToActor _asbp_first_person_character "HandGrip_R" "SnapToTarget" "SnapToTarget" "KeepWorld" true))
    (else
      (Development|PrintString "dropping")
      (Collision|SetCollisionEnabled (Variables|Default|GetSphere) "QueryAndPhysics")
      (Physics|SetSimulatePhysics (Variables|Default|GetSphere) true)
      (Transformation|DetachFromActor "KeepWorld" "KeepWorld" "KeepRelative"))))

(fn Pickup
  (params (PlayerState :type Player%20State%20Object%20Reference))
  ;[0.15 0.15 0.15 0.5] Checks if we are currently executing in the server
  (Networking|SwitchHasAuthority
    (:Authority
      ;[0.15 0.15 0.15 0.5] Checks if the object is not locked
      (if (not (Variables|Default|GetbIsLocked))
        (if (not (Variables|Default|GetbIsHeld))
          (Variables|Default|SetbIsLocked true)
          (Variables|Default|SetCurrentOwner PlayerState)
          (Variables|Default|SetbIsHeld true)
          (bind _asbp_first_person_character (Utilities|Casting|CastToBP_FirstPersonCharacter (PlayerState|GetPawn PlayerState)))
          (Variables|/Game/FirstPerson/Blueprints/BP_FirstPersonCharacter.BP_FirstPersonCharacter_C|SetHeldObject _asbp_first_person_character self)
          (Variables|Default|SetbIsLocked false))))))

(fn Drop
  (params (PlayerState :type Player%20State%20Object%20Reference))
  ;[0.15 0.15 0.15 0.5] Checks if we are currently executing in the server
  (Networking|SwitchHasAuthority
    (:Authority
      ;[0.15 0.15 0.15 0.5] Checks if the object is dropped by the player
      (if (== (Variables|Default|GetCurrentOwner) PlayerState)
        (if (Variables|Default|GetbIsHeld)
          (Variables|Default|SetbIsHeld false)
          (Variables|Default|SetCurrentOwner 0)
          (bind _asbp_first_person_character (Utilities|Casting|CastToBP_FirstPersonCharacter (PlayerState|GetPawn PlayerState)))
          (Variables|/Game/FirstPerson/Blueprints/BP_FirstPersonCharacter.BP_FirstPersonCharacter_C|SetHeldObject _asbp_first_person_character 0))))))