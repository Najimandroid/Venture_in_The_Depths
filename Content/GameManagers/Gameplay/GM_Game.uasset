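; Game mode for a multiplayer match that spawns objects, sets a money objective and decides win or loss.
; After a short delay it fills BP_FurnitureBase spawn points with random size-matched objects, forced points first, then shuffled ones up to a player-scaled count.
; The objective is 75% of the spawned value; reaching it wins, while timer expiry or all players dying loses, both returning everyone to the lobby.
; Players joining after the start are disconnected.
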(event Custom|Server_SetupAllSpawnPoints
  ;[0.15 0.15 0.15 0.5] Init Spawn Points
  (bind _outactors (Actor|GetAllActorsOfClass "/Game/GameObjects/Furnitures/BP_FurnitureBase.BP_FurnitureBase_C"))
  (for _array_element _outactors
    (for _array_element_2 (Variables|/Game/GameObjects/Furnitures/BP_FurnitureBase.BP_FurnitureBase_C|GetSpawnPoints _array_element)
      (if (.bForceSpawn (Utilities|Struct|BreakS_ObjectSpawnPoint _array_element_2))
        (Utilities|Array|Add (Variables|Default|GetSpawnPointsToUse) _array_element_2)
        (else
          (Utilities|Array|Add (Variables|Default|GetSpawnPointsAvailableToUse) _array_element_2)))))
  (CallFunction|ServerSpawnObjects (Variables|Default|GetNumberOfObjectsToSpawn)))

(event Custom|Server_SpawnObjects
  (params (NumberOfObjects :type Integer))
  ;[0.15 0.15 0.15 0.5] Spawn Objects
  ;;[0.05098 0.05098 0.05098] Firstly, spawn objects where bForceSpawn == true
  (for (_array_element _array_index) (Variables|Default|GetSpawnPointsToUse)
    (CallFunction|SpawnatPoint _array_element)
    (Utilities|Array|SetArrayElem (Variables|Default|GetSpawnPointsToUse) _array_index (Utilities|Struct|MakeS_ObjectSpawnPoint (.SpawnComponent (Utilities|Struct|BreakS_ObjectSpawnPoint _array_element)) (.AllowedSize (Utilities|Struct|BreakS_ObjectSpawnPoint _array_element)) (.RareChance (Utilities|Struct|BreakS_ObjectSpawnPoint _array_element)) (.bForceSpawn (Utilities|Struct|BreakS_ObjectSpawnPoint _array_element)) true)))
  ;;[0.05098 0.05098 0.05098] Then, the rest
  (Utilities|Array|Shuffle (Variables|Default|GetSpawnPointsAvailableToUse))
  (bind (_array_element_2 _array_index_2) (Utilities|Array|ForEachLoopwithBreak (Variables|Default|GetSpawnPointsAvailableToUse) :!label _label)
    (:LoopBody
      (if (>= (Variables|Default|GetSpawnedObjects) NumberOfObjects)
        (goto _label Break)
        (elif (== (.bAlreadyUsed (Utilities|Struct|BreakS_ObjectSpawnPoint _array_element_2)) false)
          (CallFunction|SpawnatPoint _array_element_2)
          (Utilities|Array|SetArrayElem (Variables|Default|GetSpawnPointsAvailableToUse) _array_index_2 (Utilities|Struct|MakeS_ObjectSpawnPoint (.SpawnComponent (Utilities|Struct|BreakS_ObjectSpawnPoint _array_element_2)) (.AllowedSize (Utilities|Struct|BreakS_ObjectSpawnPoint _array_element_2)) (.RareChance (Utilities|Struct|BreakS_ObjectSpawnPoint _array_element_2)) (.bForceSpawn (Utilities|Struct|BreakS_ObjectSpawnPoint _array_element_2)) true)))))
    (:Completed
      ;[0.15 0.15 0.15 0.5] Objective Price
      ;;[0.05098 0.05098 0.05098] Init Objective Price, then start the game
      (bind _output_get (Variables|Default|SetObjectivePrice (* (Variables|Default|GetObjectivePrice) 0.75)))
      (bind _asgs_game (Utilities|Casting|CastToGS_Game (Game|GetGameState)))
      (Default|InitObjectivePrice _asgs_game _output_get)
      (Default|StartGame _asgs_game))))

(event Custom|Server_StartGame
  ;[0.15 0.15 0.15 0.5] Start Game
  (Variables|Default|SetNumberOfObjectsToSpawn (* (Utilities|Array|Length (Variables|/Script/Engine.GameStateBase|GetPlayerArray (Game|GetGameState))) 8))
  (CallFunction|ServerSetupAllSpawnPoints)
  (Variables|Default|SetbHasGameStarted true))

(event Custom|Server_RegisterPlayerDeath
  ;[0.15 0.15 0.15 0.5] Check Win Condition
  (Math|Integer|IncrementInt (Variables|Default|GetDeathCounter)
    (:%20%20
      (if (>= (Variables|Default|GetDeathCounter) (Utilities|Array|Length (Variables|/Script/Engine.GameStateBase|GetPlayerArray (Game|GetGameState))))
        (Development|PrintString "Lose!" true true "(R=1.000000,G=0.136408,B=0.104890,A=1.000000)")
        (CallFunction|TeleportAllClientstoLobby)))))

(event Custom|CheckIfObjectiveReached
  (params (NewMoneyValue :type Float%20%28double-precision%29))
  ;[0.15 0.15 0.15 0.5] Game Setup
  ;;[0.05098 0.05098 0.05098] Listen To Game Events
  ;;;[0.05098 0.05098 0.05098] Listen to money change event
  (if (>= NewMoneyValue (Variables|Default|GetObjectivePrice))
    (Development|PrintString "Win!" true true "(R=1.000000,G=0.000000,B=0.628788,A=1.000000)")
    (CallFunction|TeleportAllClientstoLobby)))

(event Custom|CheckIfTimerZero
  ;[0.15 0.15 0.15 0.5] Game Setup
  ;;[0.05098 0.05098 0.05098] Listen To Game Events
  ;;;[0.05098 0.05098 0.05098] Listen to timer event
  (if (<= (Variables|/Game/GameManagers/Gameplay/GS_Game.GS_Game_C|GetRemainingTime (stale EventBeginPlay _asgs_game)) 0)
    (Development|PrintString "Lose!" true true "(R=1.000000,G=0.136408,B=0.104890,A=1.000000)")
    (CallFunction|TeleportAllClientstoLobby)))

(event EventPostLogin
  (params (NewPlayer :type Player%20Controller%20Object%20Reference))
  ;[0.15 0.15 0.15 0.5] Disconnect Players Who Arrived After The Start Of The Game
  (if (Variables|Default|GetbHasGameStarted)
    (Development|ExecuteConsoleCommand "disconnect" NewPlayer)
    (bind _asbp_first_person_player_controller (Utilities|Casting|CastToBP_FirstPersonPlayerController NewPlayer))
    (Utilities|Casting|CastToBP_FirstPersonCharacter (Pawn|GetControlledPawn _asbp_first_person_player_controller))))

(event EventBeginPlay
  ;[0.15 0.15 0.15 0.5] Game Setup
  (Utilities|FlowControl|Delay 3.0)
  (CallFunction|ServerStartGame)
  (Utilities|FlowControl|Sequence
    (:then_0
      ;;[0.05098 0.05098 0.05098] Listen To Game Events
      ;;;[0.05098 0.05098 0.05098] Listen to timer event
      (bind _asgs_game (Utilities|Casting|CastToGS_Game (Game|GetGameState)))
      (EventDispatchers|BindEventtoOnTimerUpdate _asgs_game (delegate Custom|CheckIfTimerZero))
      (Variables|/Game/GameManagers/Gameplay/GS_Game.GS_Game_C|SetRemainingTime _asgs_game (Variables|Default|GetGameTimer)))
    (:then_1
      ;;;[0.05098 0.05098 0.05098] Listen to money change event
      (bind _returnvalue (Actor|GetActorOfClass "/Game/GameObjects/Sellers/BP_ObjectSeller.BP_ObjectSeller_C"))
      (EventDispatchers|BindEventtoOnMoneyChanged _returnvalue (delegate Custom|CheckIfObjectiveReached)))))

(fn ConstructionScript
  (|CallParentFunction))

(fn SpawnatPoint
  (params (SpawnComponent :type S%20Object%20Spawn%20Point%20Structure))
  (bind (_spawncomponent _allowedsize) (Utilities|Struct|BreakS_ObjectSpawnPoint SpawnComponent))
  (bind _smallobjects (Variables|Default|GetSmallObjects))
  (bind _mediumobjects (Variables|Default|GetMediumObjects))
  (bind _largeobjects (Variables|Default|GetLargeObjects))
  (Variables|Default|SetSpawnedObjects (+ (Variables|Default|GetSpawnedObjects) 1))
  (if (Utilities|Enum|Equal(Enum) _allowedsize "NewEnumerator0")
    (Variables|Default|SetPendingObjectToBeSpawned (Utilities|ResolveSoftReference (Utilities|Set|GetItemByIndex _smallobjects (Math|Random|RandomInteger (Utilities|Set|Length _smallobjects)))))
    (elif (Utilities|Enum|Equal(Enum) _allowedsize "NewEnumerator1")
      (Variables|Default|SetPendingObjectToBeSpawned (Utilities|ResolveSoftReference (Utilities|Set|GetItemByIndex _mediumobjects (Math|Random|RandomInteger (Utilities|Set|Length _mediumobjects)))))
      (else
        (Variables|Default|SetPendingObjectToBeSpawned (Utilities|ResolveSoftReference (Utilities|Set|GetItemByIndex _largeobjects (Math|Random|RandomInteger (Utilities|Set|Length _largeobjects))))))))
  (bind _returnvalue (Game|SpawnActorfromClass (Variables|Default|GetPendingObjectToBeSpawned) (Math|Conversions|ToTransform(Vector) (Transformation|GetWorldLocation _spawncomponent)) "Undefined" "MultiplyWithRoot" 0 0))
  (if (Utilities|IsValid _returnvalue)
    (Variables|Default|SetObjectivePrice (+ (Variables|Default|GetObjectivePrice) (Variables|/Game/GameObjects/Objects/BP_HoldableObject.BP_HoldableObject_C|GetOriginPrice _returnvalue)))))

(fn TeleportAllClientstoLobby
  (for _array_element (Variables|/Script/Engine.GameStateBase|GetPlayerArray (Game|GetGameState))
    (if (Utilities|IsValid _array_element)
      (if (Utilities|IsValid (PlayerState|GetPawn _array_element))
        (bind _asbp_first_person_character (Utilities|Casting|CastToBP_FirstPersonCharacter (PlayerState|GetPawn _array_element)))
        (Default|AllClientsTeleportBacktoLobby _asbp_first_person_character)))))